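; Utility-style AI consideration that scores a context's target by its distance from the controller's pawn.
; Score divides squared Range by squared distance, avoiding a square root, then clamps to 0–1 and maps the result through ResponseCurve.
; The curve input saturates at 1 within Range and falls off with inverse-square distance beyond it.
; A missing curve, controller or target scores zero.
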(fn Score
  (params (Context :type Decision%20Context%20Structure%20%28by%20ref%29))
  (bind (_ourcontroller _ourtarget) (Utilities|Struct|BreakDecisionContext Context))
  (bind _range (Variables|Default|GetRange))
  (Utilities|IsValid (Variables|Default|GetResponseCurve)
    (:Is%20Valid
      (Utilities|IsValid _ourcontroller
        (:Is%20Valid
          (Utilities|IsValid _ourtarget
            (:Is%20Valid
              (LocalVariables|SetTarget _ourtarget)
              (LocalVariables|SetOur%20Pawn (Pawn|GetControlledPawn _ourcontroller))
              (bind _output_get (LocalVariables|SetSquare%20Range (* _range _range)))
              (return (Math|Curves|GetFloatValue (Variables|Default|GetResponseCurve) (Math|Float|Clamp(Float) (/ _output_get (Math|Vector|VectorLengthSquared (- (Transformation|GetActorLocation (LocalVariables|GetTarget)) (Transformation|GetActorLocation (LocalVariables|GetOur%20Pawn)))))))))
            (:Is%20Not%20Valid
              _)))
        (:Is%20Not%20Valid
          _)))
    (:Is%20Not%20Valid
      _))
  (return 0.0))